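; BP_GridSlot is a grid slot actor for planting that tracks whether it is free using an Available gameplay tag.
; It starts available on BeginPlay, and SetAvailability adds or removes the tag.
; When marked unavailable with a valid plant, it binds to that plant's OnDestroyed event so OnPlantHarvested can free the slot again.
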(event Custom|SetAvailability
  (params (Condition :type Boolean) (Plant :type BP%20Plant%20Object%20Reference))
  (if Condition
    ;[0.15 0.02865 0.02722 0.5] Available
    (GameplayTags|AddGameplayTag (Variables|Default|GetGameplayTags) "(TagName=\"Available\")" :!class /Script/GameplayTags.BlueprintGameplayTagLibrary)
    (else
      (Utilities|IsValid Plant
        (:Is%20Valid
          (Game|BindEventtoOnDestroyed Plant (EventDispatchers|CreateEvent :!event Custom|OnPlantHarvested)))
        (:Is%20Not%20Valid
          _))
      ;[0.15 0.02865 0.02722 0.5] Not available
      (GameplayTags|RemoveGameplayTag (Variables|Default|GetGameplayTags) "(TagName=\"Available\")" :!class /Script/GameplayTags.BlueprintGameplayTagLibrary))))

(event Custom|OnPlantHarvested
  (params (DestroyedActor :type Actor%20Object%20Reference))
  (CallFunction|SetAvailability true))

(event EventBeginPlay
  (CallFunction|SetAvailability true))

(fn ConstructionScript)