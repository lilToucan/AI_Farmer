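; BP_GridLocation is a placeable actor that spawns a grid of BP_GridSlot actors centered on its location at BeginPlay.
; GetCenter offsets the start position by half the grid span along the forward and right vectors, while CreateGrid steps slots along world X and Y by SlotSize.
; The construction script previews the layout with long-lived debug boxes, which BeginPlay flushes and CreateGrid redraws alongside each spawned slot.
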(event EventBeginPlay
  (Rendering|Debug|FlushPersistentDebugLines)
  (Variables|Default|SetStartPos (+ (Transformation|GetActorLocation) (+ (CallFunction|GetCenter (Transformation|GetActorForwardVector) (.x (Variables|Default|GetGrid%20size))) (CallFunction|GetCenter (Transformation|GetActorRightVector) (.y (Variables|Default|GetGrid%20size))))))
  (CallFunction|CreateGrid))

(event Collision|EventActorBeginOverlap
  (params (OtherActor :type Actor%20Object%20Reference)))

(event EventTick
  (params (DeltaSeconds :type Float%20%28single-precision%29)))

(fn ConstructionScript
  (Rendering|Debug|FlushPersistentDebugLines)
  (for _index (range 0 (- (.x (Variables|Default|GetGrid%20size)) 1))
    (for _index_2 (range 0 (- (.y (Variables|Default|GetGrid%20size)) 1))
      (Rendering|Debug|DrawDebugBox (+ (Math|Vector|MakeVector (* _index (Variables|Default|GetSlot%20Size)) (* _index_2 (Variables|Default|GetSlot%20Size)) 0.0) (+ (Transformation|GetActorLocation) (+ (CallFunction|GetCenter (Transformation|GetActorForwardVector) (.x (Variables|Default|GetGrid%20size))) (CallFunction|GetCenter (Transformation|GetActorRightVector) (.y (Variables|Default|GetGrid%20size)))))) (Math|Conversions|ToVector(Float) (/ (Variables|Default|GetSlot%20Size) 2.0)) "(R=0.056824,G=1.000000,B=0.071471,A=1.000000)" "0, 0, 0" 9999.0 0.0))))

(fn CreateGrid
  (for _index (range 0 (- (.x (Variables|Default|GetGrid%20size)) 1))
    (LocalVariables|SetX _index)
    (for _index_2 (range 0 (- (.y (Variables|Default|GetGrid%20size)) 1))
      (LocalVariables|SetY _index_2)
      (Game|SpawnActorfromClass "/Game/Blueprints/Actors/BP_GridSlot.BP_GridSlot_C" (Math|Transform|MakeTransform (+ (Math|Vector|MakeVector (* (LocalVariables|GetX) (Variables|Default|GetSlot%20Size)) (* (LocalVariables|GetY) (Variables|Default|GetSlot%20Size)) 0.0) (Variables|Default|GetStartPos)) "0, 0, 0" "1.000000,1.000000,1.000000") "Undefined" "MultiplyWithRoot" 0 0)
      (Rendering|Debug|DrawDebugBox (+ (Math|Vector|MakeVector (* (LocalVariables|GetX) (Variables|Default|GetSlot%20Size)) (* (LocalVariables|GetY) (Variables|Default|GetSlot%20Size)) 0.0) (Variables|Default|GetStartPos)) (Math|Conversions|ToVector(Float) (/ (Variables|Default|GetSlot%20Size) 2.0)) "(R=0.056824,G=1.000000,B=0.071471,A=1.000000)" "0, 0, 0" 9999.0 0.0))))

(fn GetCenter
  (params (A :type Vector) (InInt :type Integer))
  (return (* A (* (- (Math|Conversions|ToFloat(Integer) InInt) 1.0) -0.5 (Variables|Default|GetSlot%20Size)))))