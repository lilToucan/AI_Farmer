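; AI turret that tracks sensed actors tagged "Enemy" and can damage them.
; AI perception writes the Blackboard Target, and losing sight of an actor starts a timer that clears it after a short grace period unless an enemy is sensed again.
; ShootTarget applies damage with debug lines from two eyes, and ChangeColor tints the cube via a color map lookup, both exposed for outside callers.
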(event OnTargetPerceptionUpdated(AIPerception)
  (params (Actor :type Actor%20Object%20Reference) (Stimulus :type AI%20Stimulus%20Structure))
  (if (.bsuccessfullysensed Stimulus)
    (if (Actor|ActorHasTag Actor "Enemy")
      (AI|Components|Blackboard|SetValueasObject (AI|GetBlackboard 0) (Utilities|Name|MakeLiteralName "Target") Actor)
      (if (Utilities|Time|IsTimerActivebyHandle (Variables|Default|GetTimer))
        (Utilities|Time|ClearandInvalidateTimerbyHandle (Variables|Default|GetTimer))))
    (else
      (bind _returnvalue (Utilities|Time|SetTimerbyEvent (delegate Custom|SetTargetToNull) 3.0))
      (Variables|Default|SetTimer _returnvalue))))

(event Custom|SetTargetToNull
  (AI|Components|Blackboard|ClearValue (AI|GetBlackboard 0) (Utilities|Name|MakeLiteralName "Target")))

(fn ConstructionScript)

(fn ShootTarget
  (params (Target :type Actor%20Object%20Reference))
  (Development|PrintString "Shooting")
  (CallFunction|DrawDebugLinefromEye (Variables|Default|GetEye) Target)
  (CallFunction|DrawDebugLinefromEye (Variables|Default|GetEye2) Target)
  (Game|Damage|ApplyDamage Target 1.0 0 0))

(fn DrawDebugLinefromEye
  (params (Eye :type Scene%20Component%20Object%20Reference) (Target :type Actor%20Object%20Reference))
  (Rendering|Debug|DrawDebugLine (Transformation|GetWorldLocation Eye) (Transformation|GetActorLocation Target) "(R=0.949653,G=0.000000,B=0.000000,A=1.000000)" 0.3 3.0))

(fn ChangeColor
  (params (Color :type Name))
  (bind _colors (Variables|Default|GetColors))
  (bind (_value _returnvalue) (Utilities|Map|Find _colors Color))
  (if _returnvalue
    (LocalVariables|SetMaterialColor _value)
    (Rendering|Material|SetColorParameterValueonMaterials (Variables|Default|GetCube) "Color" (LocalVariables|GetMaterialColor))
    (return _returnvalue)
    (else
      (return _returnvalue))))