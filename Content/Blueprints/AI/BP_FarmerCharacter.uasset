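; Farmer AI character that seeds its controller's blackboard and shows a color on its cylinder mesh.
; On BeginPlay it casts to BP_FarmerController and writes the seed holder, inventory dump, inventory capacity and its current location as Home into the blackboard.
; SetCilinderColor looks up a material by key in a map and applies it to the cylinder, falling back to an error material when the key is missing.
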(event Custom|SetCilinderColor
  (params (Color :type Name))
  (bind _materials (Variables|Default|GetMaterials))
  (bind (_value _returnvalue) (Utilities|Map|Find _materials Color))
  (if _returnvalue
    (CallFunction|SetMaterialColor _value)
    (else
      (CallFunction|SetMaterialColor (.Value (Utilities|Map|Find (Variables|Default|GetMaterials) "Null/Error"))))))

(event EventBeginPlay
  (bind _asbp_farmer_controller (Utilities|Casting|CastToBP_FarmerController (Pawn|GetController)))
  (CallFunction|SetupBlackBoard (AI|GetBlackboard _asbp_farmer_controller)))

(fn ConstructionScript)

(fn SetMaterialColor
  (params (Material :type Material%20Interface%20Object%20Reference))
  (Rendering|Material|SetMaterial (Variables|Default|GetCylinder) 0 Material))

(fn SetupBlackBoard
  (params (BlackBoard :type Blackboard%20Component%20Object%20Reference))
  (Utilities|IsValid BlackBoard
    (:Is%20Valid
      (AI|Components|Blackboard|SetValueasObject BlackBoard (Utilities|Name|MakeLiteralName "SeedHolder") (Variables|Default|GetSeedHolder))
      (AI|Components|Blackboard|SetValueasObject BlackBoard (Utilities|Name|MakeLiteralName "InventoryDump") (Variables|Default|GetInventoryDump))
      (AI|Components|Blackboard|SetValueasVector BlackBoard (Utilities|Name|MakeLiteralName "Home") (Transformation|GetActorLocation))
      (Class|BlackboardComponent|SetValueasInt BlackBoard (Utilities|Name|MakeLiteralName "InventoryMax") (Variables|Default|GetInventoryMax)))))